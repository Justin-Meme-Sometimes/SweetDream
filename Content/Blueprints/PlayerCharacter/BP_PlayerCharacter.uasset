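; BP_PlayerCharacter is the first-person player character, with Enhanced Input movement gated by MovementAllowed and tap or hold crouch.
; GrabberComp grabs items from the camera's view, while InventoryComp backs the item add and use functions.
; Holding F toggles the spotlight flashlight; each press line-traces from the camera, spawning particles and damaging damageable actors.
; ChangeSanity applies deltas, calling a death stub near exactly zero, otherwise a change event.
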(event `self.ReceiveBeginPlay`
  (`EnhancedInputSubsystemInterface.AddMappingContext` (pcsubsystem `EnhancedInputLocalPlayerSubsystem` (`GameplayStatics.GetPlayerController` 0)) "/Game/Blueprints/PlayerCharacter/Input/IMC_PlayerCharacter.IMC_PlayerCharacter" 0 (struct))
  (set `self.Sanity` (`self.MaxSanity`)))

(event `EnhancedInput|/Game/Blueprints/PlayerCharacter/Input/InputActions/IA_Walk`
  (params (ActionValue :type "Vector2D Structure") (ElapsedSeconds :type "Float (double-precision)") (TriggeredSeconds :type "Float (double-precision)") (InputAction :type "InputAction Object Reference" :default "/Game/Blueprints/PlayerCharacter/Input/InputActions/IA_Walk.IA_Walk"))
  (:`Triggered`
    (if (`self.bMovementAllowed`)
      (`self.AddMovementInput` (`self.GetActorForwardVector`) ActionValue_X)
      (`self.AddMovementInput` (`self.GetActorRightVector`) ActionValue_Y))))

(event `EnhancedInput|/Game/Blueprints/PlayerCharacter/Input/InputActions/IA_Look`
  (params (ActionValue :type "Vector2D Structure") (ElapsedSeconds :type "Float (double-precision)") (TriggeredSeconds :type "Float (double-precision)") (InputAction :type "InputAction Object Reference" :default "/Game/Blueprints/PlayerCharacter/Input/InputActions/IA_Look.IA_Look"))
  (:`Triggered`
    (if (`self.bMovementAllowed`)
      (`self.AddControllerYawInput` ActionValue_X)
      (`self.AddControllerPitchInput` (* ActionValue_Y -1.0)))))

(event `EnhancedInput|/Game/Blueprints/PlayerCharacter/Input/InputActions/IA_Jump`
  (params (ActionValue :type Boolean) (ElapsedSeconds :type "Float (double-precision)") (TriggeredSeconds :type "Float (double-precision)") (InputAction :type "InputAction Object Reference" :default "/Game/Blueprints/PlayerCharacter/Input/InputActions/IA_Jump.IA_Jump"))
  (:`Started`
    (if (`self.bMovementAllowed`)
      (`self.Jump`))))

(event `EnhancedInput|/Game/Blueprints/PlayerCharacter/Input/InputActions/IA_Crouch`
  (params (ActionValue :type Boolean) (ElapsedSeconds :type "Float (double-precision)") (TriggeredSeconds :type "Float (double-precision)") (InputAction :type "InputAction Object Reference" :default "/Game/Blueprints/PlayerCharacter/Input/InputActions/IA_Crouch.IA_Crouch"))
  (bind _btaptocrouch (`self.bTapToCrouch`))
  (bind _bmovementallowed (`self.bMovementAllowed`))
  (:`Started`
    (if _bmovementallowed
      (if _btaptocrouch
        (if (`self.bIsCrouched`)
          (`self.UnCrouch`)
          (else
            (`self.Crouch`)))
        (else
          (`self.Crouch`)))))
  (:`Completed`
    (if _bmovementallowed
      (if (not _btaptocrouch)
        (`self.UnCrouch`)))))

(event `EnhancedInput|/Game/Blueprints/PlayerCharacter/Input/InputActions/IA_Interact`
  (params (ActionValue :type Boolean) (ElapsedSeconds :type "Float (double-precision)") (TriggeredSeconds :type "Float (double-precision)") (InputAction :type "InputAction Object Reference" :default "/Game/Blueprints/PlayerCharacter/Input/InputActions/IA_Interact.IA_Interact"))
  (bind _camera (`self.Camera`))
  (:`Started`
    (`/Game/Blueprints/PlayerCharacter/BP_GrabberComp.Grab Item` (`self.Grabber Comp`) (`SceneComponent.K2_GetComponentLocation` _camera) (`SceneComponent.GetForwardVector` _camera))))

(event `Key|F`
  (params (Key :type "Key Structure"))
  (bind _camera (`self.Camera`))
  (bind _returnvalue (`SceneComponent.K2_GetComponentLocation` _camera))
  ;[1 1 1] Flashlight Mechanic
  (:`Pressed`
    (`SceneComponent.ToggleVisibility` (`self.SpotLight`) false)
    (bind (_outhit _returnvalue_2) (`KismetSystemLibrary.LineTraceSingle` :`Start` _returnvalue :`End` (+ _returnvalue (* (`SceneComponent.GetForwardVector` _camera) 1000.0)) :`TraceChannel` "TraceTypeQuery2" :`DrawDebugType` "ForDuration"))
    (if _returnvalue_2
      (bind (_bblockinghit _binitialoverlap _time _distance _location _impactpoint _normal _impactnormal _physmat _hitactor) (`GameplayStatics.BreakHitResult` _outhit))
      (`GameplayStatics.SpawnEmitterAtLocation` "/Engine/Tutorial/SubEditors/TutorialAssets/TutorialParticleSystem.TutorialParticleSystem" _location (struct) (0.2 0.2 0.2) true "AutoRelease")
      (if (`Actor.bCanBeDamaged` _hitactor)
        (`GameplayStatics.ApplyDamage` _hitactor 0.5)
        (`KismetSystemLibrary.PrintString` "Applied Dmg")
        (`KismetSystemLibrary.PrintString` (`KismetSystemLibrary.GetDisplayName` _hitactor))
        (else
          (`KismetSystemLibrary.PrintString` "Actor not Hit")))))
  (:`Released`
    (`SceneComponent.ToggleVisibility` (`self.SpotLight`) false)))

(event `CharacterDeath`
  (`KismetSystemLibrary.PrintString` "you died"))

(fn `Add Item To Inventory`
  (params (`Item Name` :type Name))
  (returns (`Item Index` :type Integer))
  (bind _index (`/Game/Blueprints/PlayerCharacter/BP_InventoryComp.Add Item` (`self.Inventory Comp`) `Item Name`))
  (return _index))

(fn `ChangeSanity`
  (params (DeltaSanity :type "Float (double-precision)"))
  (bind _output_get (set `self.Sanity` (+ DeltaSanity (`self.Sanity`))))
  (if (`KismetMathLibrary.NearlyEqual_FloatFloat` _output_get)
    (`self.CharacterDeath`)
    (else
      (`self.EventChangeSanity`))))

(fn `SetMovementAllowed`
  (params (bInMovementAllowed :type Boolean))
  (bind _output_get (set `self.bMovementAllowed` bInMovementAllowed))
  (if (not _output_get)
    (`self.UnCrouch`)))

(fn `Try Use Item`
  (params (ItemName :type Name))
  (returns (wasUsed :type Boolean))
  (bind _wasremoved (`/Game/Blueprints/PlayerCharacter/BP_InventoryComp.Remove Item` (`self.Inventory Comp`) ItemName))
  (return _wasremoved))

(fn `UserConstructionScript`
  (set `/Game/Blueprints/PlayerCharacter/BP_GrabberComp.OwningActor` self (`self.Grabber Comp`)))