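; Player inventory component that stores item names in an array, using "Empty" entries as placeholder slots created at BeginPlay.
; AddItem fills the first empty slot or appends when none is free, so the inventory grows beyond its initial size.
; RemoveItem resets the first matching slot to "Empty" instead of shrinking the array.
; Changes fire the InventoryUpdated dispatcher to notify listeners.
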(event `self.ReceiveBeginPlay`
  (`self.InitializeInventory`)
  (`self.InventoryUpdated`))

(fn `Add Item`
  (params (ItemName :type Name))
  (returns (Index :type Integer))
  (locals (`Item Name` :type Name))
  (bind _inventory (`self.Inventory`))
  (bind _item_name (`local.Item Name`))
  (bind _output_get (set `local.Item Name` ItemName))
  (if (not (== _output_get "Empty"))
    (bind _index (`self.Find Item` "Empty"))
    (if (>= _index 0)
      (`KismetArrayLibrary.Array_Set` _inventory _index _item_name true)
      (`self.InventoryUpdated`)
      (return _index) ; change empty to item if empty slot exits
      (else
        _)))
  (bind _returnvalue (`KismetArrayLibrary.Array_Add` _inventory _item_name))
  (`self.InventoryUpdated`)
  (return _returnvalue))

(fn `Find Item`
  (params (`Item Name` :type Name))
  (returns (Index :type Integer))
  (return (`KismetArrayLibrary.Array_Find` (`self.Inventory`) `Item Name`)))

(fn `InitializeInventory`
  (for _ (range 5)
    (`self.Add Item` "Empty")))

(fn `Remove Item`
  (params (ItemName :type Name))
  (returns (wasRemoved :type Boolean))
  (bind _inventory (`self.Inventory`))
  (if (== ItemName "EMPTY")
    ;[1 1 1] cannot remove Empty
    (return false)
    (else
      (bind _index (`self.Find Item` ItemName))
      (if (or (>= _index (`KismetArrayLibrary.Array_Length` _inventory)) (< _index 0))
        (return false)
        (else
          (`KismetArrayLibrary.Array_Set` _inventory _index "Empty")
          (`self.InventoryUpdated`)
          (return true))))))