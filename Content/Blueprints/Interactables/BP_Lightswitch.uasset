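; BP_Lightswitch is an interactable switch that shows or hides a set of target actors.
; Each Interact event toggles IsActivated and plays the flip or unflip animation on the Switch mesh.
; It then loops over the Target array and sets each actor's hidden-in-game state to match, so targets are toggled by visibility alone.
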(event `/Game/Blueprints/Interactables/BI_Interactable.Interact`
  (params (PlayerCharacter :type "/Game/Blueprints/PlayerCharacter/BP_PlayerCharacter Object Reference"))
  (if (`self.bIsActivated`)
    (set `self.bIsActivated` false)
    (`SkeletalMeshComponent.PlayAnimation` (`self.switch`) "/Game/Assets/Lightswitch/AS_Unflip.AS_Unflip" false)
    (for _array_element (`self.Target`)
      (`self.SetActorHiddenInGame` _array_element true))
    (else
      (set `self.bIsActivated` true)
      (`SkeletalMeshComponent.PlayAnimation` (`self.switch`) "/Game/Assets/Lightswitch/AS_Flip.AS_Flip" false)
      (for _array_element_2 (`self.Target`)
        (`self.SetActorHiddenInGame` _array_element_2 false)))))

(fn `UserConstructionScript`)