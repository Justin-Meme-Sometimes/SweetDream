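; Closet interactable that lets the player hide inside and step back out.
; Interact toggles on IsPlayerHiding: entering stores the player, disables movement, teleports them to the Closet component and aligns control rotation with the actor.
; Exiting re-enables movement, places the player just in front and clears the reference.
; The Box switches its Pawn response to Overlap on entry and Block on exit.
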(event `/Game/Blueprints/Interactables/BI_Interactable.Interact`
  (params (PlayerCharacter :type "/Game/Blueprints/PlayerCharacter/BP_PlayerCharacter Object Reference"))
  (bind _bisplayerhiding (`self.bIsPlayerHiding`))
  (bind _player (`self.Player`))
  (`PrimitiveComponent.SetCollisionResponseToChannel` (`self.Box`) "ECC_Pawn" (select `bool` _bisplayerhiding :`false` "ECR_Overlap" :`true` "ECR_Block" :!type "ECollisionResponse Enum"))
  (if _bisplayerhiding
    (`/Game/Blueprints/PlayerCharacter/BP_PlayerCharacter.SetMovementAllowed` _player true)
    (`self.K2_SetActorLocation` _player (+ (`SceneComponent.K2_GetComponentLocation` (`self.closet`)) (* (`self.GetActorForwardVector`) 80.0)) false false)
    (set `self.bIsPlayerHiding` false)
    (set `self.Player` null)
    (else
      (`/Game/Blueprints/PlayerCharacter/BP_PlayerCharacter.SetMovementAllowed` PlayerCharacter false)
      (bind _output_get (set `self.Player` PlayerCharacter))
      (`self.K2_SetActorLocation` _output_get (`SceneComponent.K2_GetComponentLocation` (`self.closet`)) false false)
      (`Controller.SetControlRotation` (`Pawn.GetController` _output_get) (`self.K2_GetActorRotation`))
      (set `self.bIsPlayerHiding` true))))

(fn `UserConstructionScript`)