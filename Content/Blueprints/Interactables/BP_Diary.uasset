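; BP_Diary is an interactable diary that shows a DiaryImage widget on screen.
; Actor overlap enables input and copies its ImageVal to the player character's Imageindex, presumably selecting the image shown.
; While input is enabled, R uses a FlipFlop to create or remove the widget.
; Ending overlap disables input and removes any open widget, without resetting the FlipFlop.
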(event `Key|R`
  (params (Key :type "Key Structure"))
  (:`Pressed`
    (`/Engine/EditorBlueprintResources/StandardMacros.FlipFlop`
      (:`A`
        (bind _returnvalue (`|CreateWidget` "/Game/Assets/Widgets/DiaryImage.DiaryImage_C"))
        (`UserWidget.AddToViewport` _returnvalue 0))
      (:`B`
        (`/Engine/EditorBlueprintResources/StandardMacros.IsValid` _returnvalue :!label _label
          (:`Is Valid`
            (`Widget.RemoveFromParent` _returnvalue)))))))

(event `self.ReceiveActorBeginOverlap`
  (params (OtherActor :type "Actor Object Reference"))
  (`self.EnableInput` (`GameplayStatics.GetPlayerController` 0))
  (bind _asbp_player_character (cast `/Game/Blueprints/PlayerCharacter/BP_PlayerCharacter` (`GameplayStatics.GetPlayerCharacter` 0)))
  (set `/Game/Blueprints/PlayerCharacter/BP_PlayerCharacter.imageindex` (`self.image_val`) _asbp_player_character))

(event `self.ReceiveActorEndOverlap`
  (params (OtherActor :type "Actor Object Reference"))
  (`self.DisableInput` null)
  (goto _label))

(fn `UserConstructionScript`)