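; Mover_BP is an actor that moves toward a configurable Moving offset.
; On BeginPlay it feeds its InterpToMovement component two control points flagged as relative: the actor's world location and the Moving vector.
; When OnTouch is set, any actor overlap also eases the StaticMesh to Moving as a relative location through MoveComponentTo.
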(event `self.ReceiveBeginPlay`
  (bind _interptomovement (`self.InterpToMovement`))
  (`InterpToMovementComponent.AddControlPointPosition` _interptomovement (`self.K2_GetActorLocation`) true)
  (`InterpToMovementComponent.AddControlPointPosition` _interptomovement (`self.moving`) true))

(event `self.ReceiveActorBeginOverlap`
  (params (OtherActor :type "Actor Object Reference"))
  (if (`self.OnTouch`)
    (`KismetSystemLibrary.MoveComponentTo` (`self.StaticMesh`) (`self.moving`) (struct) true true 0.2 true)))

(fn `UserConstructionScript`)