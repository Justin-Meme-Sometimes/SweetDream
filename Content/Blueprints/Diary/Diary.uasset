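; Diary actor that stores collected page textures and shows them to the player in a UMG widget.
; Read creates a DisplayDiary_Widget, adds it to the viewport and sets its Page image to the current page.
; Flip shifts the page index by an increment without bounds checks, Add appends a new page, and Close removes the widget.
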(event `Read`
  (bind _returnvalue (`|CreateWidget` "/Game/Blueprints/Diary/DisplayDiary_Widget.DisplayDiary_Widget_C"))
  (bind _output_get (set `self.diary_widget` _returnvalue))
  (`UserWidget.AddToViewport` _output_get 0)
  (`Image.SetBrushFromTexture` (`/Game/Blueprints/Diary/DisplayDiary_Widget.Page` _returnvalue) (`|GetArrayItem` (`self.pages`) (`self.PageNumber`)) false))

(event `Flip`
  (params (Increment :type Integer))
  (set `self.PageNumber` (+ (`self.PageNumber`) Increment))
  (`Image.SetBrushFromTexture` (`/Game/Blueprints/Diary/DisplayDiary_Widget.Page` (`self.diary_widget`)) (`|GetArrayItem` (`self.pages`) (`self.PageNumber`)) false))

(event `Add`
  (params (newPage :type "Texture2D Object Reference"))
  (`KismetArrayLibrary.Array_Add` (`self.pages`) newPage))

(event `Close`
  (`Widget.RemoveFromParent` (`self.diary_widget`)))

(fn `UserConstructionScript`)