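; Inventory system Blueprint that currently handles look-at detection for interaction, with AddInventory left as an empty stub.
; Every Tick, InteractionTrace sphere-traces forward from the player camera manager up to InteractionRange, ignoring its owner.
; A newly hit actor is cached as LookAtActor and its LookAtMessage result is printed on screen.
; The cache clears when nothing is hit, so messages print only when the target changes.
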(event `self.ReceiveTick`
  (params (DeltaSeconds :type "Float (single-precision)"))
  (`self.InteractionTrace`))

(fn `AddInventory`)

(fn `InteractionTrace`
  (bind _returnvalue (`GameplayStatics.GetPlayerCameraManager` 0))
  (bind _returnvalue_2 (`self.K2_GetActorLocation` _returnvalue))
  (bind (_outhit _returnvalue_3) (`KismetSystemLibrary.SphereTraceSingle` _returnvalue_2 (+ _returnvalue_2 (* (`SceneComponent.GetForwardVector` (`PlayerCameraManager.TransformComponent` _returnvalue)) (`self.InteractionRange`))) 15.0 "TraceTypeQuery3" false (`|MakeArray` (`self.GetOwner`))))
  (if _returnvalue_3
    (bind (_bblockinghit _binitialoverlap _time _distance _location _impactpoint _normal _impactnormal _physmat _hitactor) (`GameplayStatics.BreakHitResult` _outhit))
    (if (!= _hitactor (`self.Look At Actor`))
      (bind _output_get (set `self.Look At Actor` _hitactor))
      (bind _message (message `/Game/Inventory/IInteractInterface.LookAt` _output_get))
      (`KismetSystemLibrary.PrintString` _message))
    (else
      (set `self.Look At Actor` null))))

(fn `UserConstructionScript`)