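; Zombie enemy Blueprint that handles damage, fleeing and death, passing state to its Enemy_Controller's Blackboard.
; Each hit removes fixed health; low health or detected light sets the Flee key.
; At zero health, it plays a standing or non-standing death montage, then ragdolls and stops AI logic.
; Tick restores full health and clears Flee whenever regeneration is allowed; the sound update function is empty.
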(event `self.ReceiveAnyDamage`
  (params (Damage :type "Float (single-precision)") (DamageType :type "DamageType Object Reference") (InstigatedBy :type "Controller Object Reference") (DamageCauser :type "Actor Object Reference"))
  (bind _mesh (`self.Mesh`))
  (`KismetSystemLibrary.PrintString` "Enemy Dmgsed")
  (bind _output_get (set `self.EnemyHealth` (- (`self.EnemyHealth`) 0.2)))
  (`KismetSystemLibrary.PrintString` (`KismetStringLibrary.Conv_DoubleToString` _output_get))
  (if (<= _output_get 0.5)
    (`KismetSystemLibrary.PrintString` "Flee")
    (`BlackboardComponent.SetValueAsBool` (`AIController.Blackboard` (`self.control`)) "Flee" true))
  (if (<= _output_get 0.0)
    (`KismetSystemLibrary.PrintString` "Killed Enemy")
    (if (`self.IsStanding`)
      (if (not (`self.IsDying`))
        (`|PlayMontage` _mesh "/Game/Blueprints/Enemy/Animations/NoFaceAnimations/zombie_death_Montage.zombie_death_Montage" 0.5
          (:`then`
            (set `self.IsDying` true))
          (:`OnCompleted`
            (`PrimitiveComponent.SetSimulatePhysics` (`self.Mesh`) true :!label _label)
            (`BrainComponent.StopLogic` (`AIController.BrainComponent` (`self.control`)) ""))
          (:`OnBlendOut`
            (set `self.IsDying` false))))
      (elif (not (`self.IsDying`))
        (`|PlayMontage` _mesh "/Game/Blueprints/Enemy/Animations/NoFaceAnimations/zombie_dying_Montage.zombie_dying_Montage" 0.5
          (:`then`
            (set `self.IsDying` true))
          (:`OnCompleted`
            (goto _label))
          (:`OnBlendOut`
            (set `self.IsDying` false)))))))

(event `self.ReceiveBeginPlay`
  (bind _asenemy_controller (cast `/Game/Blueprints/Enemy/Enemy_Controller` (`self.GetController`)))
  (set `self.control` _asenemy_controller))

(event `self.ReceiveTick`
  (params (DeltaSeconds :type "Float (single-precision)"))
  (`self.RegainHeath`))

(event `LightDetected`
  (`BlackboardComponent.SetValueAsBool` (`AIController.Blackboard` (`self.control`)) "Flee" true))

(fn `RegainHeath`
  (if (`self.CanRegainHealth`)
    (set `self.EnemyHealth` 1.0)
    (`BlackboardComponent.SetValueAsBool` (`AIController.Blackboard` (`self.control`)) "Flee" false)))

(fn `StandingWalking/Transition`
  (if (>= (`BlackboardComponent.GetValueAsFloat` (`AIController.Blackboard` (`self.control`)) "DistanceToPlayer") (`self.MaxDistanceBeforeTransition`))
    (set `self.IsStanding` false)))

(fn `Update Sound`
  (params (`New State` :type "/Game/Blueprints/Enemy/EnemyAnimNotifys/NoFace/AN_States_NoFace Enum" :default "NewEnumerator0")))

(fn `UserConstructionScript`)