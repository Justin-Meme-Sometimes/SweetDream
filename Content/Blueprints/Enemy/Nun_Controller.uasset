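; AI controller for the Nun enemy that runs BT_Nun and feeds it player perception and range data through the blackboard.
; Sight updates the target only while the player is moving and unhidden, storing last known location on loss.
; HandleSoundSense processes prediction and HandlePredictionSense processes hearing, opposite to their names.
; Tick writes attack range and distance using Player, which hearing sets and sight clears.
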(event `self.ReceiveBeginPlay`
  (`self.RunBehaviorTree` "/Game/Blueprints/Enemy/BT_Nun.BT_Nun")
  (`self.InitalizeBlackboard`)
  (bind _asbp_player_character (cast `/Game/Blueprints/PlayerCharacter/BP_PlayerCharacter` (`GameplayStatics.GetPlayerCharacter` 0)))
  (set `self.checkPlayer` _asbp_player_character))

(event `self.ReceiveTick`
  (params (DeltaSeconds :type "Float (single-precision)"))
  (`self.IsInAttackRange`))

(event `self.AIPerception.OnTargetPerceptionUpdated`
  (params (Actor :type "Actor Object Reference") (Stimulus :type "AIStimulus Structure"))
  (`self.HandleSightSense` Actor Stimulus)
  (`self.HandleSoundSense` Stimulus Actor)
  (`self.HandlePredictionSense` Stimulus Actor))

(fn `HandleGroupSense`
  (params (Stimulus :type "AIStimulus Structure"))
  (bind _returnvalue (`AIPerceptionSystem.GetSenseClassForStimulus` Stimulus))
  (if (not (== _returnvalue "/Script/AIModule.AISense_Team"))
    (return)))

(fn `HandlePredictionSense`
  (params (Stimulus :type "AIStimulus Structure") (actor :type "Actor Object Reference"))
  (bind (_age _expirationage _strength _stimuluslocation _receiverlocation _tag _bsuccessfullysensed) (break `AIStimulus` (`local.Stimulus`)))
  (bind _returnvalue (`KismetMathLibrary.SelectObject` (`GameplayStatics.GetPlayerCharacter` 0) null _bsuccessfullysensed))
  (bind _returnvalue_2 (`AIPerceptionSystem.GetSenseClassForStimulus` Stimulus))
  (if (== _returnvalue_2 "/Script/AIModule.AISense_Hearing")
    (if (== (`local.Actor`) (`GameplayStatics.GetPlayerCharacter` 0))
      (bind _asactor (cast `Actor` _returnvalue))
      (set `self.Player` _asactor)
      (`BlackboardComponent.SetValueAsObject` (`self.Blackboard`) "TargetActor" _returnvalue)
      (if (not _bsuccessfullysensed)
        (`BlackboardComponent.SetValueAsVector` (`self.Blackboard`) "LastKnownLocation" _stimuluslocation))
      (else
        (return)))
    (else
      (return))))

(fn `HandleSightSense`
  (params (Actor :type "Actor Object Reference") (Stimulus :type "AIStimulus Structure"))
  (bind (_stimulus_age _stimulus_expirationage _stimulus_strength _stimulus_stimuluslocation _stimulus_receiverlocation _stimulus_tag _stimulus_bsuccessfullysensed) (break `AIStimulus` (`local.Stimulus`)))
  (bind _checkplayer (`self.checkPlayer`))
  (if (`/Game/Blueprints/PlayerCharacter/BP_PlayerCharacter.isHiding` _checkplayer)
    _
    (elif (not (<= (`KismetMathLibrary.VSize` (`self.GetVelocity` _checkplayer)) 10.0))
      (bind _returnvalue (`AIPerceptionSystem.GetSenseClassForStimulus` Stimulus))
      (if (== _returnvalue "/Script/AIModule.AISense_Sight")
        (if (== (`local.Actor`) (`GameplayStatics.GetPlayerCharacter` 0))
          (set `self.Player` null)
          (`BlackboardComponent.SetValueAsObject` (`self.Blackboard`) "TargetActor" (`KismetMathLibrary.SelectObject` (`GameplayStatics.GetPlayerCharacter` 0) null _stimulus_bsuccessfullysensed))
          (if (not _stimulus_bsuccessfullysensed)
            (`BlackboardComponent.SetValueAsVector` (`self.Blackboard`) "LastKnownLocation" _stimulus_stimuluslocation))
          (else
            (return)))
        (else
          (return))))))

(fn `HandleSoundSense`
  (params (Stimulus :type "AIStimulus Structure") (Actor :type "Actor Object Reference"))
  (bind (_age _expirationage _strength _stimuluslocation _receiverlocation _tag _bsuccessfullysensed) (break `AIStimulus` (`local.Stimulus`)))
  (bind _returnvalue (`AIPerceptionSystem.GetSenseClassForStimulus` Stimulus))
  (if (== _returnvalue "/Script/AIModule.AISense_Prediction")
    (if (== (`local.Actor`) (`GameplayStatics.GetPlayerCharacter` 0))
      (if _bsuccessfullysensed
        (`BlackboardComponent.SetValueAsVector` (`self.Blackboard`) "LastKnownLocation" _stimuluslocation))
      (else
        (return)))
    (else
      (return))))

(fn `InitalizeBlackboard`
  (`BlackboardComponent.SetValueAsVector` (`self.Blackboard`) "SpawnLocation" (`self.K2_GetActorLocation`))
  (`BlackboardComponent.SetValueAsBool` (`self.Blackboard`) "Flee" false))

(fn `IsInAttackRange`
  (bind _blackboard (`self.Blackboard`))
  (bind _player (`self.Player`))
  (bind _returnvalue (`KismetMathLibrary.VSize` (- (`self.K2_GetActorLocation` (`self.K2_GetPawn`)) (`self.K2_GetActorLocation` _player))))
  (bind _returnvalue_2 (<= _returnvalue (`self.Attack Range`)))
  (`/Engine/EditorBlueprintResources/StandardMacros.IsValid` _player
    (:`Is Valid`
      (`KismetSystemLibrary.PrintString` (`KismetStringLibrary.Conv_BoolToString` _returnvalue_2))
      (`BlackboardComponent.SetValueAsBool` _blackboard "InRange" _returnvalue_2)
      (`BlackboardComponent.SetValueAsFloat` _blackboard "DistanceToPlayer" _returnvalue))))

(fn `UserConstructionScript`)