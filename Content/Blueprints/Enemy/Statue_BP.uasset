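; Enemy statue Blueprint that reacts when the player character overlaps it, setting off a field effect and a change in the nun.
; On overlap it spawns an FS_MasterField at its Mother component's location, sets the activation type and fires CETrigger, likely to fracture the statue.
; It then calls Transition on the first Nun_BP found in the level, with no guard against repeated overlaps.
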(event `self.ReceiveActorBeginOverlap`
  (params (OtherActor :type "Actor Object Reference"))
  (cast `/Game/Blueprints/PlayerCharacter/BP_PlayerCharacter` OtherActor)
  (bind _returnvalue (`|SpawnActorFromClass` "/Engine/EditorResources/FieldNodes/FS_MasterField.FS_MasterField_C" (`KismetMathLibrary.MakeTransform` (`SceneComponent.K2_GetComponentLocation` (`self.Mother`))) "Undefined" "MultiplyWithRoot" null null))
  (set `/Engine/EditorResources/FieldNodes/FS_MasterField.ActivationType` "NewEnumerator4" _returnvalue)
  (`/Engine/EditorResources/FieldNodes/FS_MasterField.CE_Trigger` _returnvalue)
  (bind _outactors (`GameplayStatics.GetAllActorsOfClass` "/Game/Blueprints/Enemy/Nun_BP.Nun_BP_C"))
  (bind _output (`|GetArrayItem` _outactors))
  (`/Engine/EditorBlueprintResources/StandardMacros.IsValid` _output
    (:`Is Valid`
      (`/Game/Blueprints/Enemy/Nun_BP.Transition` _output))))

(fn `UserConstructionScript`)