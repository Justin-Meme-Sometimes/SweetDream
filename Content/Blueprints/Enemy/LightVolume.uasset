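; LightVolume is an enemy-related spotlight actor that can sweep and flicker.
; When Moving is set, RotateBase recursively eases LightBase between two opposite rotations with pauses.
; Tick uses delays to randomly blink the SpotLight off briefly when DoesFlicker is set.
; DetectEnemy debug-traces for pawns along the beam but is never called here, and overlap handling only casts without acting.
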(event `self.ReceiveBeginPlay`
  (`LocalLightComponent.SetAttenuationRadius` (`self.SpotLight`) (`self.attenuation`))
  (if (`self.moving`)
    (`self.rotateBase`)))

(event `self.ReceiveTick`
  (params (DeltaSeconds :type "Float (single-precision)"))
  (`KismetSystemLibrary.Delay` 1.0)
  (`self.flicker` false)
  (`KismetSystemLibrary.Delay` 0.1)
  (`SceneComponent.SetVisibility` (`self.SpotLight`) true false))

(event `rotateBase`
  (bind _lightbase (`self.LightBase`))
  (bind _lightbase_2 (`self.LightBase`))
  (`KismetSystemLibrary.MoveComponentTo` _lightbase (`SceneComponent.RelativeLocation` _lightbase) (struct :`Yaw` 40.0) true true 5.0 true)
  (`KismetSystemLibrary.Delay` 2.0)
  (`KismetSystemLibrary.MoveComponentTo` _lightbase_2 (`SceneComponent.RelativeLocation` _lightbase_2) (struct :`Yaw` -40.0) true true 5.0 true)
  (`KismetSystemLibrary.Delay` 2.0)
  (`self.rotateBase`))

(event `self.ReceiveActorBeginOverlap`
  (params (OtherActor :type "Actor Object Reference"))
  (cast `/Game/Blueprints/Enemy/EnemyAI_BP` OtherActor
    (:`CastFailed`
      (cast `/Game/Blueprints/Enemy/Nun_BP` _))))

(fn `detectEnemy`
  (bind _spotlight (`self.SpotLight`))
  (bind _returnvalue (`SceneComponent.K2_GetComponentLocation` _spotlight))
  (bind (_outhit _returnvalue_2) (`KismetSystemLibrary.LineTraceSingleForObjects` _returnvalue (+ (* (`SceneComponent.GetForwardVector` _spotlight) (`LocalLightComponent.AttenuationRadius` _spotlight)) _returnvalue) (`|MakeArray` "ObjectTypeQuery3" :!type "EObjectTypeQuery Enum") false (`|MakeArray` (`GameplayStatics.GetPlayerPawn` 0) :!type "Actor Object Reference") "ForDuration"))
  (if _returnvalue_2
    (`KismetSystemLibrary.PrintString` "Called")
    (`KismetSystemLibrary.PrintString` (`KismetSystemLibrary.GetDisplayName` (`.HitActor` (`GameplayStatics.BreakHitResult` _outhit))))))

(fn `EnemyEnterLightVolume`)

(fn `flicker`
  (params (visible :type Boolean))
  (if (`KismetMathLibrary.RandomBool`)
    (if (`self.doesFlicker`)
      (`SceneComponent.SetVisibility` (`self.SpotLight`) false false))))

(fn `moveLight`)

(fn `UserConstructionScript`)